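; Player controller that steers the WineChar pawn toward the mouse cursor.
; On BeginPlay it caches the controlled WineChar, then each Tick sets its yaw toward a point projected a fixed distance along the deprojected cursor ray.
; It also adds local pitch from world X velocity scaled by RotationSpeed.
; The Forward/Backward axis moves the pawn along that same cursor-facing yaw.
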(event EventBeginPlay
  (bind _aswine_char (Utilities|Casting|CastToWineChar (Pawn|GetControlledPawn)))
  (Variables|Default|SetPlayerRef _aswine_char))

(event EventTick
  (params (DeltaSeconds :type Float%20%28single-precision%29))
  (bind (_worldlocation _worlddirection) (Game|Player|ConvertMouseLocationToWorldSpace))
  (bind _playerref (Variables|Default|GetPlayerRef))
  ;[1 1 1] Character mouse rotation
  (Transformation|SetActorRotation _playerref (Math|Rotator|MakeRotator 0.0 0.0 (.Yaw (Math|Rotator|BreakRotator (Math|Rotator|FindLookatRotation (Transformation|GetActorLocation _playerref) (+ _worldlocation (* _worlddirection 2.5e+02)))))))
  (Transformation|AddActorLocalRotation (Variables|Default|GetPlayerRef) (Math|Rotator|MakeRotator 0.0 (* (.X (Math|Vector|BreakVector (Transformation|GetVelocity (Variables|Default|GetPlayerRef)))) (Variables|Default|Getrotation%20speed)) 0.0) false false))

(event Input|AxisEvents|InputAxisForward/Backward
  (params (AxisValue :type Float%20%28single-precision%29))
  (bind (_worldlocation _worlddirection) (Game|Player|ConvertMouseLocationToWorldSpace))
  (bind _playerref (Variables|Default|GetPlayerRef))
  ;[1 1 1] Character Movement
  (Pawn|Input|AddMovementInput _playerref (Math|Vector|GetForwardVector (Math|Rotator|MakeRotator 0.0 0.0 (.Yaw (Math|Rotator|BreakRotator (Math|Rotator|FindLookatRotation (Transformation|GetActorLocation _playerref) (+ _worldlocation (* _worlddirection 2.5e+02))))))) AxisValue false))

(fn ConstructionScript)