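; CabbageGameMode is a game mode that runs the level's countdown timer and triggers the fail state when time runs out.
; Tick feeds a one-second Delay, so TotalSeconds and Seconds drop about once per second, with Seconds rolling over into Minutes.
; When Minutes and Seconds both reach zero, it shows the FailedLvl_T widget, plays the lose sound and switches to UI-only input with a visible cursor.
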(event EventTick
  (params (DeltaSeconds :type Float%20%28single-precision%29))
  (bind _returnvalue (Game|GetPlayerController 0))
  ;[1 1 1] count down timer
  (Utilities|FlowControl|Delay 1.0)
  (Variables|Default|Settotal_seconds (- (Variables|Default|Gettotal_seconds) 1))
  (Variables|Default|Setseconds (- (Variables|Default|Getseconds) 1))
  (if (< (Variables|Default|Getseconds) 0)
    (Variables|Default|Setminutes (- (Variables|Default|Getminutes) 1))
    (Variables|Default|Setseconds 59))
  ;[1 1 1] game over condition
  (if (== (Variables|Default|Getminutes) 0)
    (if (== (Variables|Default|Getseconds) 0)
      (bind _returnvalue_2 (UserInterface|CreateWidget "/Game/Menu/FailedLvl_T.FailedLvl_T_C"))
      (Audio|PlaySoundatLocation "/Game/audio/lose_Cue.lose_Cue" "0, 0, 0" "0, 0, 0" 1.0 1.0 0.0 0 0 0)
      (UserInterface|Viewport|AddtoViewport _returnvalue_2 0)
      (Input|SetInputModeUIOnly _returnvalue 0 "DoNotLock")
      (Variables|/Script/Engine.PlayerController|SetbShowMouseCursor _returnvalue true))))

(fn ConstructionScript)