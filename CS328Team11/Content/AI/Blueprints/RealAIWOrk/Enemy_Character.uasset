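; Enemy character Blueprint that damages the Cabbage actor on contact and can be destroyed by damage.
; A hit on Cabbage applies damage, then shows the FailedLvl_E fail menu with the mouse cursor.
; Incoming damage lowers CurrentHP; at zero or below the enemy destroys itself and also opens that fail menu.
; A helper function sets the character's max walk speed.
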(event Collision|EventHit
  (params (MyComp :type Primitive%20Component%20Object%20Reference) (Other :type Actor%20Object%20Reference) (OtherComp :type Primitive%20Component%20Object%20Reference) (bSelfMoved :type Boolean) (HitLocation :type Vector :default "0, 0, 0") (HitNormal :type Vector :default "0, 0, 0") (NormalImpulse :type Vector :default "0, 0, 0") (Hit :type Hit%20Result%20Structure%20%28by%20ref%29))
  ;[1 1 1] Damage
  (bind _ascabbage (Utilities|Casting|CastToCabbage Other))
  (Game|Damage|ApplyDamage _ascabbage (Variables|Default|GetDamage) 0 0)
  ;[1 1 1] For Fail Menu
  (bind _returnvalue (UserInterface|CreateWidget "/Game/Menu/FailedLvl_E.FailedLvl_E_C"))
  (UserInterface|Viewport|AddtoViewport _returnvalue 0)
  (Variables|/Script/Engine.PlayerController|SetbShowMouseCursor (Game|GetPlayerController 0) true))

(event Game|Damage|EventAnyDamage
  (params (Damage :type Float%20%28single-precision%29) (DamageType :type Damage%20Type%20Object%20Reference) (InstigatedBy :type Controller%20Object%20Reference) (DamageCauser :type Actor%20Object%20Reference))
  ;[1 1 1] Damage
  (Variables|Default|SetCurrent%20HP (- (Variables|Default|GetCurrent%20HP) Damage))
  (if (<= (Variables|Default|GetCurrent%20HP) 0.0)
    (Actor|DestroyActor)
    ;[1 1 1] For Fail Menu
    (bind _returnvalue (UserInterface|CreateWidget "/Game/Menu/FailedLvl_E.FailedLvl_E_C"))
    (UserInterface|Viewport|AddtoViewport _returnvalue 0)
    (Variables|/Script/Engine.PlayerController|SetbShowMouseCursor (Game|GetPlayerController 0) true)))

(fn ConstructionScript)

(fn UpdateWalkSpeed
  (params (NewWalkSpeed :type Float%20%28single-precision%29))
  (Variables|/Script/Engine.CharacterMovementComponent|SetMaxWalkSpeed (Variables|Character|GetCharacterMovement) NewWalkSpeed))