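; Customer2_3 is an AI customer pawn that patrols the level, damages any Cabbage it hits and can be destroyed.
; On BeginPlay, chained AI MoveTo calls visit four target points with short pauses, then a Patrol event loops the route; a failed move ends it.
; Incoming damage reduces CurrentHP and destroys the actor at zero or below.
; Unconnected three-target and two-target patrol variants remain in the graph.
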(event Custom|patrol
  ;[1 1 1] 4x targets
  (AI|AIMoveTo self "0, 0, 0" (Variables|Default|GetTargetPoint1) 5.0 false
    (:OnSuccess
      (Utilities|FlowControl|Delay 0.2)
      (AI|AIMoveTo self "0, 0, 0" (Variables|Default|GetTargetPoint2) 5.0 false
        (:OnSuccess
          (Utilities|FlowControl|Delay 0.2)
          (AI|AIMoveTo self "0, 0, 0" (Variables|Default|GetTargetPoint3) 5.0 false
            (:OnSuccess
              (Utilities|FlowControl|Delay 0.2)
              (AI|AIMoveTo self "0, 0, 0" (Variables|Default|GetTargetPoint4) 5.0 false
                (:OnSuccess
                  (CallFunction|Patrol))))))))))

(event Collision|EventHit
  (params (MyComp :type Primitive%20Component%20Object%20Reference) (Other :type Actor%20Object%20Reference) (OtherComp :type Primitive%20Component%20Object%20Reference) (bSelfMoved :type Boolean) (HitLocation :type Vector :default "0, 0, 0") (HitNormal :type Vector :default "0, 0, 0") (NormalImpulse :type Vector :default "0, 0, 0") (Hit :type Hit%20Result%20Structure%20%28by%20ref%29))
  ;[1 1 1] Damage
  (bind _ascabbage (Utilities|Casting|CastToCabbage Other))
  (Game|Damage|ApplyDamage _ascabbage (Variables|Default|GetDamage) 0 0))

(event Game|Damage|EventAnyDamage
  (params (Damage :type Float%20%28single-precision%29) (DamageType :type Damage%20Type%20Object%20Reference) (InstigatedBy :type Controller%20Object%20Reference) (DamageCauser :type Actor%20Object%20Reference))
  ;[1 1 1] Damage
  (Variables|Default|SetCurrentHP (- (Variables|Default|GetCurrentHP) Damage))
  (if (<= (Variables|Default|GetCurrentHP) 0.0)
    (Actor|DestroyActor)))

(event EventBeginPlay
  ;[1 1 1] 4x targets
  (AI|AIMoveTo self "0, 0, 0" (Variables|Default|GetTargetPoint1) 5.0 false
    (:OnSuccess
      (Utilities|FlowControl|Delay 0.2)
      (AI|AIMoveTo self "0, 0, 0" (Variables|Default|GetTargetPoint2) 5.0 false
        (:OnSuccess
          (Utilities|FlowControl|Delay 0.2)
          (AI|AIMoveTo self "0, 0, 0" (Variables|Default|GetTargetPoint3) 5.0 false
            (:OnSuccess
              (Utilities|FlowControl|Delay 0.2)
              (AI|AIMoveTo self "0, 0, 0" (Variables|Default|GetTargetPoint4) 5.0 false
                (:OnSuccess
                  (CallFunction|Patrol))))))))))

(fn ConstructionScript)